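; BP_PlayerCharacter is the player character Blueprint, turning Enhanced Input actions into looking, movement and arm use.
; Look input drives controller yaw and inverted pitch.
; Move input applies movement along forward and right vectors built from the control yaw only, so camera pitch does not affect direction.
; The left and right arm actions forward to separate use-arm calls, and the construction script is empty.
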(event `EnhancedInput|/Game/Player/Input/IA_Look`
  (params (ActionValue :type "Vector2D Structure") (ElapsedSeconds :type "Float (double-precision)") (TriggeredSeconds :type "Float (double-precision)") (InputAction :type "InputAction Object Reference" :default "/Game/Player/Input/IA_Look.IA_Look"))
  (bind (_x _y) (`KismetMathLibrary.BreakVector2D` ActionValue))
  (:`Triggered`
    (`self.AddControllerYawInput` _x)
    (`self.AddControllerPitchInput` (- 0.0 _y))))

(event `EnhancedInput|/Game/Player/Input/IA_Move`
  (params (ActionValue :type "Vector2D Structure") (ElapsedSeconds :type "Float (double-precision)") (TriggeredSeconds :type "Float (double-precision)") (InputAction :type "InputAction Object Reference" :default "/Game/Player/Input/IA_Move.IA_Move"))
  (bind (_x _y) (`KismetMathLibrary.BreakVector2D` ActionValue))
  (bind _returnvalue (`KismetMathLibrary.MakeRotator` 0.0 0.0 (.yaw (`self.GetControlRotation`))))
  (:`Triggered`
    (`self.AddMovementInput` (`KismetMathLibrary.GetForwardVector` _returnvalue) _y)
    (`self.AddMovementInput` (`KismetMathLibrary.GetRightVector` _returnvalue) _x)))

(event `EnhancedInput|/Game/Player/Input/IA_UseArmL`
  (params (ActionValue :type Boolean) (ElapsedSeconds :type "Float (double-precision)") (TriggeredSeconds :type "Float (double-precision)") (InputAction :type "InputAction Object Reference" :default "/Game/Player/Input/IA_UseArmL.IA_UseArmL"))
  (:`Triggered`
    (`self.Use Arm L`)))

(event `EnhancedInput|/Game/Player/Input/IA_UseArmR`
  (params (ActionValue :type Boolean) (ElapsedSeconds :type "Float (double-precision)") (TriggeredSeconds :type "Float (double-precision)") (InputAction :type "InputAction Object Reference" :default "/Game/Player/Input/IA_UseArmR.IA_UseArmR"))
  (:`Triggered`
    (`self.Use Arm R`)))

(fn `UserConstructionScript`)